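; Mine is an interactable explosive actor that detonates when anything begins overlapping its Sphere component.
; It applies point damage to the overlapping actor, using a scaled direction away from the mine and a synthetic hit result on the spine_01 bone.
; It then spawns an explosion particle effect and sound at its location and destroys itself.
; There is no filtering of the overlapping actor and no area damage.
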(event OnComponentBeginOverlap(Sphere)
  (params (OverlappedComponent :type Primitive%20Component%20Object%20Reference) (OtherActor :type Actor%20Object%20Reference) (OtherComp :type Primitive%20Component%20Object%20Reference) (OtherBodyIndex :type Integer) (bFromSweep :type Boolean) (SweepResult :type Hit%20Result%20Structure%20%28by%20ref%29))
  (bind _returnvalue (Transformation|GetActorLocation))
  (bind _output_get (Variables|Default|SetHitDirection (* (Math|Vector|Normalize (- (Transformation|GetActorLocation OtherActor) (Transformation|GetActorLocation))) 10000)))
  (Game|Damage|ApplyPointDamage OtherActor (Variables|Default|GetDamage) _output_get (Collision|MakeHitResult false false 0.0 0.0 "0, 0, 0" "0, 0, 0" "0,0,1" "0,0,1" 0 0 0 "spine_01"))
  (Effects|SpawnEmitteratLocation "/Game/Download/StarterContent/Particles/P_Explosion.P_Explosion" _returnvalue "0, 0, 0" "2.000000,2.000000,2.000000")
  (Audio|SpawnSoundatLocation "/Game/Download/StarterContent/Audio/Explosion02.Explosion02" _returnvalue "0, 0, 0" 1.0 1.0 0.0 0 0)
  (Actor|DestroyActor))

(fn ConstructionScript)