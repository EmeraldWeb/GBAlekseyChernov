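; HoverPlatform is a physics-driven actor that hovers its static mesh above surfaces beneath it.
; Each Tick, a short-radius sphere trace runs downward from the mesh against WorldStatic and PhysicsBody objects.
; On a hit, it applies upward force scaled by HoverPower and closeness to the surface, as a mass-independent acceleration change.
; An alternative line trace with debug drawing remains in the graph but never runs.
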(event EventBeginPlay)

(event Collision|EventActorBeginOverlap
  (params (OtherActor :type Actor%20Object%20Reference)))

(event EventTick
  (params (DeltaSeconds :type Float%20%28single-precision%29))
  (bind _staticmesh (Variables|Default|GetStaticMesh))
  (bind _returnvalue (Transformation|GetWorldLocation _staticmesh))
  (bind (_outhit _returnvalue_2) (Collision|SphereTraceForObjects _returnvalue (+ _returnvalue "0, 0,-1000.000000") 15.0 (Utilities|Array|MakeArray "ObjectTypeQuery1" "ObjectTypeQuery4") false 0 "None"))
  (if _returnvalue_2
    ;[1 1 1] Функция добавляет к компоненту силу
    (Physics|AddForce (Variables|Default|GetStaticMesh) (Math|Vector|MakeVector 0.0 0.0 (* (- 1.0 (.Time (Collision|BreakHitResult _outhit))) (Variables|Default|GetHoverPower))) "None" true)))

(fn ConstructionScript)