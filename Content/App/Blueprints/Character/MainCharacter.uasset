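; Player character with movement, look, run, health and interaction with lamps and weapons.
; Capsule overlaps track nearby BaseLamp and BaseWeapon references; Interact toggles lamps or swaps the weapon attached at WeaponPlace, which can fire or drop with physics.
; Point damage multiplies headshots and sets a flag blocking generic damage, cleared only after a lethal hit.
; Death ragdolls the mesh along the hit direction, disables movement and drops the weapon.
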(event OnComponentBeginOverlap(CapsuleComponent)
  (params (OverlappedComponent :type Primitive%20Component%20Object%20Reference) (OtherActor :type Actor%20Object%20Reference) (OtherComp :type Primitive%20Component%20Object%20Reference) (OtherBodyIndex :type Integer) (bFromSweep :type Boolean) (SweepResult :type Hit%20Result%20Structure%20%28by%20ref%29))
  (Utilities|FlowControl|Sequence
    (:then_0
      ;[1 1 1] Cast - уточнение типа данных.  Каст это функция которая делает попытку привести один тип данных к другому типу данных. На входе ссылка на родительский объект/класс, на выходе ссылка на дочерний объект/класс.
      (bind _asbase_lamp (Utilities|Casting|CastToBaseLamp OtherActor))
      (Variables|Default|SetLampReference _asbase_lamp))
    (:then_1
      (bind _asbase_weapon (Utilities|Casting|CastToBaseWeapon OtherActor))
      (Variables|Default|SetWeaponRefInteract _asbase_weapon))))

(event OnComponentEndOverlap(CapsuleComponent)
  (params (OverlappedComponent :type Primitive%20Component%20Object%20Reference) (OtherActor :type Actor%20Object%20Reference) (OtherComp :type Primitive%20Component%20Object%20Reference) (OtherBodyIndex :type Integer))
  (Utilities|FlowControl|Sequence
    (:then_0
      (bind _asbase_lamp (Utilities|Casting|CastToBaseLamp OtherActor))
      (if (== _asbase_lamp (Variables|Default|GetLampReference))
        (Variables|Default|SetLampReference 0)))
    (:then_1
      (bind _asbase_weapon (Utilities|Casting|CastToBaseWeapon OtherActor))
      (if (== _asbase_weapon (Variables|Default|GetWeaponRefInteract))
        (Variables|Default|SetWeaponRefInteract 0)))))

(event Custom|InitCharacter
  (Variables|Default|SetHP_Current (Variables|Default|GetHP_Max)))

(event Custom|Death
  (Utilities|FlowControl|DoOnce false
    (:Completed
      (Physics|SetSimulatePhysics (Variables|Character|GetMesh) true)
      (Physics|AddImpulse (Variables|Character|GetMesh) (Variables|Default|GetHitDirection) (Variables|Default|GetHitBone) false)
      (Pawn|Components|CharacterMovement|DisableMovement (Variables|Character|GetCharacterMovement))
      (CallFunction|DropItem))))

(event EventBeginPlay
  (CallFunction|InitCharacter))

(event Game|Damage|EventAnyDamage
  (params (Damage :type Float%20%28single-precision%29) (DamageType :type Damage%20Type%20Object%20Reference) (InstigatedBy :type Controller%20Object%20Reference) (DamageCauser :type Actor%20Object%20Reference))
  (if (not (Variables|Default|GetHasPointDamage))
    (bind _characterdead (CallFunction|ApplyDamage Damage))
    (if _characterdead
      (CallFunction|Death))))

(event Game|Damage|EventPointDamage
  (params (Damage :type Float%20%28single-precision%29) (DamageType :type Damage%20Type%20Object%20Reference) (HitLocation :type Vector :default "0, 0, 0") (HitNormal :type Vector :default "0, 0, 0") (HitComponent :type Primitive%20Component%20Object%20Reference) (BoneName :type Name :default "None") (ShotFromDirection :type Vector :default "0, 0, 0") (InstigatedBy :type Controller%20Object%20Reference) (DamageCauser :type Actor%20Object%20Reference) (HitInfo :type Hit%20Result%20Structure%20%28by%20ref%29))
  (Variables|Default|SetHitDirection ShotFromDirection)
  (Variables|Default|SetHasPointDamage true)
  (bind _output_get (Variables|Default|SetHitBone (.HitBoneName (Collision|BreakHitResult HitInfo))))
  (if (Utilities|Name|Equal(Name) _output_get "head")
    (bind _characterdead (CallFunction|ApplyDamage (* Damage (Variables|Default|GetCriticalMultiply))))
    (Development|PrintString "HEADSHOT!" true true "(R=1.000000,G=0.000000,B=0.024208,A=1.000000)" 5.0)
    (else
      (bind _characterdead_2 (CallFunction|ApplyDamage Damage))))
  (if (or _characterdead _characterdead_2)
    (CallFunction|Death)
    (Utilities|FlowControl|Delay 0.2)
    (Variables|Default|SetHasPointDamage false)))

(event Input|ActionEvents|InputActionInteract
  (params (Key :type Key%20Structure :default "None"))
  (:Pressed
    (Development|PrintString "Press \"E\""))
  (:Released
    (Development|PrintString "Release \"E\"")))

(event Input|ActionEvents|InputActionRun
  (params (Key :type Key%20Structure :default "None"))
  (bind _charactermovement (Variables|Character|GetCharacterMovement))
  (:Pressed
    (Variables|/Script/Engine.CharacterMovementComponent|SetMaxWalkSpeed _charactermovement 3e+03))
  (:Released
    (Variables|/Script/Engine.CharacterMovementComponent|SetMaxWalkSpeed _charactermovement 6e+02)))

(event Input|ActionEvents|InputActionInteract
  (params (Key :type Key%20Structure :default "None"))
  (bind _lampreference (Variables|Default|GetLampReference))
  (:Pressed
    (Utilities|FlowControl|Sequence
      (:then_0
        ;[1 1 1] Проверка на валидность ссылки
        (if (Utilities|IsValid (Variables|Default|GetLampReference))
          (Default|SwitchLight _lampreference (not (Variables|/Game/App/Blueprints/Interact/BaseLamp.BaseLamp_C|GetOn/Off _lampreference)))))
      (:then_1
        (if (Utilities|IsValid (Variables|Default|GetWeaponRefInteract))
          (if (Utilities|IsValid (Variables|Default|GetWeaponRefActive))
            (CallFunction|DropItem)
            (CallFunction|TakeItem)
            (else
              (CallFunction|TakeItem))))))))

(event Input|ActionEvents|InputActionFire
  (params (Key :type Key%20Structure :default "None"))
  (bind _weaponrefactive (Variables|Default|GetWeaponRefActive))
  (:Pressed
    (if (Utilities|IsValid _weaponrefactive)
      (Default|FireBaseWeapon _weaponrefactive))))

(event Input|ActionEvents|InputActionDropItem
  (params (Key :type Key%20Structure :default "None"))
  (:Pressed
    (CallFunction|DropItem)))

(event Input|AxisEvents|InputAxisTurn
  (params (AxisValue :type Float%20%28single-precision%29))
  (Pawn|Input|AddControllerYawInput AxisValue))

(event Input|AxisEvents|InputAxisMoveRight
  (params (AxisValue :type Float%20%28single-precision%29))
  (Pawn|Input|AddMovementInput (Transformation|GetActorRightVector) AxisValue false))

(event Input|AxisEvents|InputAxisMoveForward
  (params (AxisValue :type Float%20%28single-precision%29))
  (Pawn|Input|AddMovementInput (Transformation|GetActorForwardVector) AxisValue false))

(event Input|AxisEvents|InputAxisLookUp
  (params (AxisValue :type Float%20%28single-precision%29))
  (Pawn|Input|AddControllerPitchInput AxisValue))

(fn ConstructionScript)

(fn NewFunction0)

(fn DropItem
  (if (Utilities|IsValid (Variables|Default|GetWeaponRefActive))
    (Transformation|DetachFromActor (Variables|Default|GetWeaponRefActive) "KeepWorld" "KeepWorld" "KeepWorld")
    (Physics|SetSimulatePhysics (Variables|/Game/App/Blueprints/Weapon/BaseWeapon.BaseWeapon_C|GetStaticMesh (Variables|Default|GetWeaponRefActive)) true)
    (Variables|Default|SetWeaponRefActive 0)))

(fn TakeItem
  (Variables|Default|SetWeaponRefActive (Variables|Default|GetWeaponRefInteract))
  (Transformation|AttachComponentToComponent (Variables|Default|GetWeaponRefActive) (Variables|Default|GetWeaponPlace) "None" "SnapToTarget" "SnapToTarget" "KeepWorld" true)
  (Physics|SetSimulatePhysics (Variables|/Game/App/Blueprints/Weapon/BaseWeapon.BaseWeapon_C|GetStaticMesh (Variables|Default|GetWeaponRefInteract)) false)
  (Variables|Default|SetWeaponRefInteract 0))

(fn ApplyDamage
  (params (B :type Float%20%28single-precision%29))
  (bind _output_get (Variables|Default|SetHP_Current (Math|Float|Clamp(Float) (- (Variables|Default|GetHP_Current) B) 0.0 (Variables|Default|GetHP_Max))))
  (return (== _output_get 0.0)))