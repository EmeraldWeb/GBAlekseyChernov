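; Laser gun weapon that deals continuous damage along a straight beam while firing is active.
; The FireBaseWeapon override only sets IsActive, leaving the parent's fire logic unconnected.
; While active, Tick line-traces forward from SpawnShellPlace with debug drawing and applies frame-time-scaled damage to the hit actor.
; Particles and audio run only during a hit, with the particles moved to the impact point.
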(event EventFireBaseWeapon
  (params (Activate :type Boolean))
  ;[1 1 1] Перегрузка родительской функции
  (Variables|Default|SetIsActive Activate))

(event EventTick
  (params (DeltaSeconds :type Float%20%28single-precision%29))
  (bind _spawnshellplace (Variables|Default|GetSpawnShellPlace))
  (bind _particlesystem (Variables|Default|GetParticleSystem))
  (bind _returnvalue (Transformation|GetWorldLocation _spawnshellplace))
  (|CallParentFunction DeltaSeconds)
  (if (Variables|Default|GetIsActive)
    (bind (_outhit _returnvalue_2) (Collision|LineTraceForObjects _returnvalue (+ _returnvalue (* (Math|Vector|GetForwardVector (Variables|Default|GetSpawnShellPlace)) (Variables|Default|GetDistance))) (Utilities|Array|MakeArray "ObjectTypeQuery1" "ObjectTypeQuery3" "ObjectTypeQuery4" "ObjectTypeQuery5" "ObjectTypeQuery6") false 0 "ForOneFrame"))
    (if _returnvalue_2
      (Components|Activation|Activate _particlesystem false)
      (Variables|Default|SetWeaponDamage 25.0)
      (Game|Damage|ApplyDamage (.HitActor (Collision|BreakHitResult _outhit)) (* (Variables|Default|GetWeaponDamage) (Utilities|Time|GetWorldDeltaSeconds)) 0 0)
      (Transformation|SetWorldLocation (Variables|Default|GetParticleSystem) (.ImpactPoint (Collision|BreakHitResult _outhit)) false false)
      (else
        (Components|Activation|Deactivate _particlesystem)))
    (else
      (Components|Activation|Deactivate (Variables|Default|GetParticleSystem)))))

(fn ConstructionScript
  (|CallParentFunction))