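; Player controller that owns the main UI and manages the player character's game-over and restart cycle.
; BeginPlay creates MainWindow and caches the pawn as MainCharacter.
; Tick polls it to push HP and interact prompts (weapon name or "Activate") and to trigger game over with UI-only input at zero HP.
; Restart resets the UI, spawns a fresh MainCharacter at the first PlayerStart found, possesses it and restores game input.
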(event Custom|Restart
  (Class|WidgetSwitcher|SetActiveWidgetIndex (Variables|/Game/App/UIX/MainWindow.MainWindow_C|GetMainSwitcher (Variables|Default|GetMainWindow)))
  (bind _outactors (Actor|GetAllActorsOfClass "/Script/Engine.PlayerStart"))
  (bind _returnvalue (Game|SpawnActorfromClass "/Game/App/Blueprints/Character/MainCharacter.MainCharacter_C" (Transformation|GetActorTransform (Utilities|Array|Get(acopy) _outactors)) "Undefined" 0 0))
  (Variables|Default|SetMyPawnRef _returnvalue)
  (Pawn|UnPossess)
  (Pawn|Possess (Variables|Default|GetMyPawnRef))
  (Input|SetInputModeGameOnly self)
  (Variables|Default|SetAlive true)
  (Variables|Default|SetbShowMouseCursor false))

(event EventBeginPlay
  (Utilities|FlowControl|Sequence
    (:then_0
      ;[1 1 1] Создаем виджет
      (bind _returnvalue (UserInterface|CreateWidget "/Game/App/UIX/MainWindow.MainWindow_C"))
      ;[1 1 1] Записываем ссылку на виджет в переменную
      (bind _output_get (Variables|Default|SetMainWindow _returnvalue))
      ;[1 1 1] Добавляем на экран
      (UserInterface|Viewport|AddtoViewport _output_get 0))
    (:then_1
      (bind _asmain_character (Utilities|Casting|CastToMainCharacter (Pawn|GetControlledPawn)))
      (Variables|Default|SetMyPawnRef _asmain_character))))

(event EventTick
  (params (DeltaSeconds :type Float%20%28single-precision%29))
  (if (Utilities|IsValid (Variables|Default|GetMyPawnRef))
    (Utilities|FlowControl|Sequence
      (:then_0
        (|SetHP))
      (:then_1
        (|UpdateInteractInfo))
      (:then_2
        (if (Variables|Default|GetAlive)
          (if (<= (Variables|/Game/App/Blueprints/Character/MainCharacter.MainCharacter_C|GetHP_Current (Variables|Default|GetMyPawnRef)) 0.0)
            (Variables|Default|SetAlive false)
            (Default|GameOver (Variables|Default|GetMainWindow))
            (Variables|Default|SetbShowMouseCursor true)
            (Input|SetInputModeUIOnly self (Variables|Default|GetMainWindow) "DoNotLock")))))))

(fn ConstructionScript)