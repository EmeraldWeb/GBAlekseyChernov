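; AI controller that arms its AI_Character with a random weapon on possess and runs patrol, chase and fire combat.
; Perception sets any sensed MainCharacter on another team as the focused Enemy and clears it when lost.
; Tick, rather than a behavior tree, picks timed bursts within FireDistance, chasing beyond it, or patrol without an enemy.
; Patrol visits random target points from the pawn's list, falling back to all MyTargetPoint actors.
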(event OnTargetPerceptionUpdated(AIPerception)
  (params (Actor :type Actor%20Object%20Reference) (Stimulus :type AI%20Stimulus%20Structure))
  (if (.bSuccessfullySensed (Utilities|Struct|BreakAIStimulus Stimulus))
    (bind _asmain_character (Utilities|Casting|CastToMainCharacter Actor))
    (if (not (== (Variables|/Game/App/Blueprints/Character/MainCharacter.MainCharacter_C|GetMyTeam _asmain_character) (Variables|/Game/App/Blueprints/Character/MainCharacter.MainCharacter_C|GetMyTeam (Variables|Default|GetMyControlledPawn))))
      (bind _output_get (Variables|Default|SetEnemy _asmain_character))
      (AI|SetFocus _output_get))
    (elif (== Actor (Variables|Default|GetEnemy))
      (bind _output_get_2 (Variables|Default|SetEnemy 0))
      (AI|SetFocus _output_get_2))))

(event Custom|MoveToTP
  (bind _mycontrollertp (Variables|Default|GetMyControllerTP))
  ;[1 1 1] Патрулирование
  (if (not (Variables|Default|GetOnPatrol))
    (Variables|Default|SetOnPatrol true)
    (AI|AIMoveTo (Variables|Default|GetMyControlledPawn) "0, 0, 0" (Utilities|Array|Get(acopy) _mycontrollertp (Math|Random|RandomIntegerinRange 0 (Utilities|Array|LastIndex _mycontrollertp))) 5.0 false
      (:OnSuccess
        _)
      (:OnFail
        _))
    (Utilities|FlowControl|Delay 3.0)
    (Variables|Default|SetOnPatrol false)))

(event Custom|ChaseToEnemy
  ;[1 1 1] Погоня за врагом
  (AI|AIMoveTo (Variables|Default|GetMyControlledPawn) "0, 0, 0" (Variables|Default|GetEnemy) 6e+02 false))

(event Custom|Fire
  (if (not (Variables|Default|GetOnFire))
    (Variables|Default|SetOnFire true)
    (Default|Fire (Variables|Default|GetMyControlledPawn) true)
    (Utilities|FlowControl|Delay 2.0)
    (Default|Fire (Variables|Default|GetMyControlledPawn) false)
    (Utilities|FlowControl|Delay 1.0)
    (Variables|Default|SetOnFire false)))

(event EventPossess
  (params (PossessedPawn :type Pawn%20Object%20Reference))
  (bind _weaponarray (Variables|Default|GetWeaponArray))
  (bind _asai_character (Utilities|Casting|CastToAI_Character (Pawn|GetControlledPawn)))
  (Variables|Default|SetMyControlledPawn _asai_character)
  (bind _returnvalue (Game|SpawnActorfromClass (Utilities|Array|Get(acopy) _weaponarray (Math|Random|RandomIntegerinRange 0 (Utilities|Array|LastIndex _weaponarray))) (Transformation|GetActorTransform (Variables|Default|GetMyControlledPawn)) "AlwaysSpawn" 0 0))
  (Variables|/Game/App/Blueprints/Character/MainCharacter.MainCharacter_C|SetWeaponRefInteract (Variables|Default|GetMyControlledPawn) _returnvalue)
  (Default|TakeItem (Variables|Default|GetMyControlledPawn))
  (if (> (Utilities|Array|Length (Variables|/Game/App/Blueprints/AI/AI_Character.AI_Character_C|GetMyTP (Variables|Default|GetMyControlledPawn))) 0)
    (Variables|Default|SetMyControllerTP (Variables|/Game/App/Blueprints/AI/AI_Character.AI_Character_C|GetMyTP (Variables|Default|GetMyControlledPawn)))
    (else
      ;[1 1 1] Возвращает экземпляры всеъ экземпляров Класса
      (bind _outactors (Actor|GetAllActorsOfClass "/Game/App/Blueprints/AI/MyTargetPoint.MyTargetPoint_C"))
      (Variables|Default|SetMyControllerTP _outactors)))
  (CallFunction|MovetoTP))

(event EventTick
  (params (DeltaSeconds :type Float%20%28single-precision%29))
  (bind _enemy (Variables|Default|GetEnemy))
  (bind _returnvalue (Utilities|IsValid _enemy))
  (Variables|/Game/App/Blueprints/Character/MainCharacter.MainCharacter_C|SetOnAim (Variables|Default|GetMyControlledPawn) _returnvalue)
  (if _returnvalue
    (if (< (Transformation|GetDistanceTo (Variables|Default|GetMyControlledPawn) (Variables|Default|GetEnemy)) (Variables|Default|GetFireDistance))
      (CallFunction|Fire)
      (else
        (CallFunction|ChasetoEnemy)))
    (else
      (CallFunction|MovetoTP))))

(fn ConstructionScript)