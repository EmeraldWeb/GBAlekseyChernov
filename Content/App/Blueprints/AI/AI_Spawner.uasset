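; AI spawner that keeps up to a set maximum of AI pawns of a configurable class alive in the level.
; Every tick it checks its tracked pawn list and, while below the limit, spawns one pawn at its Arrow component's location.
; Each new pawn is added to the list and bound to a destroyed callback that removes it, so losses are refilled without delay.
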(event Custom|SpawnAI
  (if (< (Utilities|Array|Length (Variables|Default|GetMyPawns)) (Variables|Default|GetMaxAI))
    (bind _returnvalue (AI|SpawnAIFromClass (Variables|Default|GetMyAIClass) 0 (Transformation|GetWorldLocation (Variables|Default|GetArrow)) "0, 0, 0" false 0))
    (Utilities|Array|AddUnique (Variables|Default|GetMyPawns) _returnvalue)
    (Game|BindEventtoOnDestroyed _returnvalue (delegate Custom|CustomEvent_0))))

(event Custom|CustomEvent_0
  (params (DestroyedActor :type Actor%20Object%20Reference))
  (bind _aspawn (Utilities|Casting|CastToPawn DestroyedActor))
  (Utilities|Array|RemoveItem (Variables|Default|GetMyPawns) _aspawn))

(event EventTick
  (params (DeltaSeconds :type Float%20%28single-precision%29))
  (CallFunction|SpawnAI))

(fn ConstructionScript)